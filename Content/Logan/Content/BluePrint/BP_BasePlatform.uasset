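; Base platform Blueprint with six directional faces (Up, Down, Left, Right, Front, Back), each given its own dynamic material instance on BeginPlay.
; ReduceColor is a timer-style step that writes a time-mapped scalar to the face material picked by ColorActivated, apparently to fade its color.
; Its parameter and timer function names are unset, and nothing in this graph calls it.
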(event EventBeginPlay
  (bind _returnvalue (Rendering|Material|CreateDynamicMaterialInstance (Variables|Default|GetUp) 0 0 "None" :!class /Script/Engine.PrimitiveComponent))
  (Variables|Default|SetUpMat _returnvalue)
  (bind _returnvalue_2 (Rendering|Material|CreateDynamicMaterialInstance (Variables|Default|GetDown) 0 0 "None" :!class /Script/Engine.PrimitiveComponent))
  (Variables|Default|SetDownMat _returnvalue_2)
  (bind _returnvalue_3 (Rendering|Material|CreateDynamicMaterialInstance (Variables|Default|GetLeft) 0 0 "None" :!class /Script/Engine.PrimitiveComponent))
  (Variables|Default|SetLeftMat _returnvalue_3)
  (bind _returnvalue_4 (Rendering|Material|CreateDynamicMaterialInstance (Variables|Default|GetRight) 0 0 "None" :!class /Script/Engine.PrimitiveComponent))
  (Variables|Default|SetRightMat _returnvalue_4)
  (bind _returnvalue_5 (Rendering|Material|CreateDynamicMaterialInstance (Variables|Default|GetFront) 0 0 "None" :!class /Script/Engine.PrimitiveComponent))
  (Variables|Default|SetFrontMat _returnvalue_5)
  (bind _returnvalue_6 (Rendering|Material|CreateDynamicMaterialInstance (Variables|Default|GetBack) 0 0 "None" :!class /Script/Engine.PrimitiveComponent))
  (Variables|Default|SetBackMat _returnvalue_6))

(fn ConstructionScript)

(fn ReduceColor
  (bind _coloractivated (Variables|Default|GetColorActivated))
  (bind _outmat (Utilities|SelectMaterial _coloractivated))
  (bind _returnvalue (Rendering|Material|GetScalarParameterValue _outmat "None" :!class /Script/Engine.MaterialInstanceDynamic))
  (if (<= _returnvalue 0.0)
    (Utilities|Time|ClearTimerbyFunctionName 0 "")
    (else
      (Variables|Default|SetLerpDuration (+ (Variables|Default|GetLerpTimer) (Utilities|Time|GetWorldDeltaSeconds)))
      (Rendering|Material|SetScalarParameterValue _outmat "None" (Math|Float|MapRangeClamped (Variables|Default|GetLerpTimer) 0.0 (Variables|Default|GetLerpDuration) 0.0 0.0) :!class /Script/Engine.MaterialInstanceDynamic))))