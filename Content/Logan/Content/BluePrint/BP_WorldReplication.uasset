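; BP_WorldReplication tiles the world at BeginPlay by spawning copies of WorldRootActor's class in a 3D grid; it is spatial duplication, with no networking shown.
; One loop over Row × Col × Height uses VectorByCubeGrid to turn each index into a WorldSize-spaced offset roughly centered on the root.
; Each copy takes the root's rotation and scale and attaches to WorldRootGhost with KeepRelative rules.
; Debug box drawing is present but disconnected.
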(event EventBeginPlay
  (bind _worldrootactor (Variables|Default|GetWorldRootActor))
  (bind _returnvalue (Transformation|GetActorTransform _worldrootactor))
  (for _index (range 0 (- (* (Variables|Default|GetRow) (Variables|Default|GetCol) (Variables|Default|GetHeight)) 1))
    (bind _returnvalue_2 (Game|SpawnActorfromClass (Utilities|GetClass _worldrootactor) (Math|Transform|MakeTransform (+ (Math|Vector|MakeVector (.X (Utilities|VectorbyCubeGrid _index)) (.Y (Utilities|VectorbyCubeGrid _index)) (.Z (Utilities|VectorbyCubeGrid _index))) (.location _returnvalue)) (.rotation _returnvalue) (.scale _returnvalue)) "AlwaysSpawn" "MultiplyWithRoot" 0 0))
    (Transformation|AttachActorToActor _returnvalue_2 (Variables|Default|GetWorldRootGhost) "None" "KeepRelative" "KeepRelative" "KeepRelative" true)))

(fn ConstructionScript)