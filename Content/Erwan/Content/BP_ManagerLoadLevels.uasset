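; Level streaming manager that loads and unloads sublevels at runtime.
; On BeginPlay it asynchronously streams in two map levels and makes them visible, then binds its Load and Unload events to the game instance.
; Those events stream a level in or out by name without blocking, with a debug print on load.
; The LoadLevel function is an empty stub.
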(event Custom|Load
  (params (LevelName :type Name))
  (Development|PrintString "LoadLevel")
  (Game|LoadStreamLevel(byName) LevelName true))

(event Custom|Unload
  (params (LevelName :type Name))
  (Game|UnloadStreamLevel(byName) LevelName false))

(event EventBeginPlay
  (Class|GameplayStatics|LoadStreamLevelbySoftObjectPtr "/Game/Erwan/Content/Level/LV_Map1.LV_Map1" true false)
  (Class|GameplayStatics|LoadStreamLevelbySoftObjectPtr "/Game/Erwan/Content/Level/LV_Map2.LV_Map2" true false)
  (bind _asbp_game_instance (Utilities|Casting|CastToBP_GameInstance (Game|GetGameInstance)))
  (EventDispatchers|BindEventtoLoadLevel _asbp_game_instance (delegate Custom|Load))
  (EventDispatchers|BindEventtoUnloadLevel _asbp_game_instance (delegate Custom|Unload)))

(fn ConstructionScript)

(fn LoadLevel
  (params (LevelName :type Name :default "None")))