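; Pawn that runs custom directional gravity, world-bound checks and on-screen helper hints.
; Looping timers call the gravity and bounds functions, which are defined outside these graphs.
; SetupWidget adds the helper and VHS overlay widgets, and runs from both the construction script and BeginPlay.
; A timeline fades the wall hint at start, while a detection trigger toggles the grab-cube hint for actors tagged Interactable.
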(event OnComponentBeginOverlap(DetectTrigger)
  (params (OverlappedComponent :type Primitive%20Component%20Object%20Reference) (OtherActor :type Actor%20Object%20Reference) (OtherComp :type Primitive%20Component%20Object%20Reference) (OtherBodyIndex :type Integer) (bFromSweep :type Boolean) (SweepResult :type Hit%20Result%20Structure%20%28by%20ref%29))
  (if (Actor|ActorHasTag OtherActor "Interactable")
    (Default|HelperGrabCubeVisible (Variables|Default|GetWidgetHelper))))

(event OnComponentEndOverlap(DetectTrigger)
  (params (OverlappedComponent :type Primitive%20Component%20Object%20Reference) (OtherActor :type Actor%20Object%20Reference) (OtherComp :type Primitive%20Component%20Object%20Reference) (OtherBodyIndex :type Integer))
  (if (Actor|ActorHasTag OtherActor "Interactable")
    (Default|HelperGrabCubeInvisible (Variables|Default|GetWidgetHelper) 0.0)))

(event Custom|CustomGravity
  (Class|CPPPawn|AddDirectionalGravity (Variables|Default|GetGravityDt)))

(event Custom|CheckWorldBound
  (Class|CPPPawn|CheckWorldBounds))

(event EventBeginPlay
  (Utilities|SetupWidget)
  (Utilities|Time|SetTimerbyEvent (delegate Custom|CheckWorldBound) 0.1 true)
  (Utilities|Time|SetTimerbyEvent (delegate Custom|CustomGravity) (Variables|Default|GetGravityDt) true)
  (Default|HelperWallVisible (Variables|Default|GetWidgetHelper))
  (bind _opacityvalue (Timeline|Timeline Play)
    (:Update
      (Default|HelperWallInvisible (Variables|Default|GetWidgetHelper) _opacityvalue))))

(fn ConstructionScript
  (Utilities|SetupWidget))