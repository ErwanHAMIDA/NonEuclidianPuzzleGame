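; BP_ColliderLoadLevel is a trigger actor that requests level loading and unloading when any actor overlaps it.
; On BeginPlay it caches the BP_GameInstance, which receives both requests by level name.
; An overlap loads LoadLevelName, waits a second, then unloads UnloadLevelName, skipping either step if its name is None.
; Its own LoadLevel function is an empty stub.
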(event Collision|EventActorBeginOverlap
  (params (OtherActor :type Actor%20Object%20Reference))
  (if (== (Variables|Default|GetLoadLevelName) "None")
    _
    (else
      (Default|CallLoadLevel (Variables|Default|GetGameInstance) (Variables|Default|GetLoadLevelName))
      (Utilities|FlowControl|Delay 1.0)))
  (if (not (== (Variables|Default|GetUnloadLevelName) "None"))
    (Default|CallUnloadLevel (Variables|Default|GetGameInstance) (Variables|Default|GetUnloadLevelName))))

(event EventBeginPlay
  (bind _asbp_game_instance (Utilities|Casting|CastToBP_GameInstance (Game|GetGameInstance)))
  (Variables|Default|SetGameInstance _asbp_game_instance))

(fn ConstructionScript)

(fn LoadLevel
  (params (LevelName :type Name :default "None")))