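; BP_SwitchGravityZone is a trigger zone that switches gravity for actors entering it.
; On begin overlap, it passes WhereSwitchGravity through ChangeGravityMessage to any actor implementing BPI_CanChangeGravity.
; A single IsAlreadyPlayedSound flag limits the 2D trigger cue to one play until any such actor ends overlap, which resets it.
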(event Collision|EventActorEndOverlap
  (params (OtherActor :type Actor%20Object%20Reference))
  (if (Utilities|DoesObjectImplementInterface OtherActor "/Game/Erwan/Content/Interfaces/BPI_CanChangeGravity.BPI_CanChangeGravity_C")
    (Variables|Default|SetIsAlreadyPlayedSound false)))

(event Collision|EventActorBeginOverlap
  (params (OtherActor :type Actor%20Object%20Reference))
  (if (Utilities|DoesObjectImplementInterface OtherActor "/Game/Erwan/Content/Interfaces/BPI_CanChangeGravity.BPI_CanChangeGravity_C")
    (Class|BPICanChangeGravity|ChangeGravity(Message) OtherActor (Variables|Default|GetWhereSwitchGravity))
    (if (not (Variables|Default|GetIsAlreadyPlayedSound))
      (Audio|PlaySound2D "/Game/Erwan/Content/Audio/Cue/GravityTriggerZoneCue.GravityTriggerZoneCue" 1.0 1.0 0.0 0 0)
      (Variables|Default|SetIsAlreadyPlayedSound true))))

(fn ConstructionScript)