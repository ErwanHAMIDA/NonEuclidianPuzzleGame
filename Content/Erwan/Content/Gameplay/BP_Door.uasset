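; BP_Door is an indexed door that dithers away and destroys itself when opened.
; On BeginPlay it applies a dynamic dithering material and binds to the game instance's open-door event.
; A matching index plays a sound and a timeline that drives the material's Percent parameter before destruction.
; A box trigger shows or hides the open-door helper widget on the overlapping BP_Character.
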(event OnComponentBeginOverlap(Box)
  (params (OverlappedComponent :type Primitive%20Component%20Object%20Reference) (OtherActor :type Actor%20Object%20Reference) (OtherComp :type Primitive%20Component%20Object%20Reference) (OtherBodyIndex :type Integer) (bFromSweep :type Boolean) (SweepResult :type Hit%20Result%20Structure%20%28by%20ref%29))
  (bind _asbp_character (Utilities|Casting|CastToBP_Character OtherActor))
  (Default|HelperOpenDoorVisible (Variables|/Game/Erwan/Content/BP_Character.BP_Character_C|GetWidgetHelper _asbp_character)))

(event OnComponentEndOverlap(Box)
  (params (OverlappedComponent :type Primitive%20Component%20Object%20Reference) (OtherActor :type Actor%20Object%20Reference) (OtherComp :type Primitive%20Component%20Object%20Reference) (OtherBodyIndex :type Integer))
  (bind _asbp_character (Utilities|Casting|CastToBP_Character OtherActor))
  (Default|HelperOpenDoorInvisible (Variables|/Game/Erwan/Content/BP_Character.BP_Character_C|GetWidgetHelper _asbp_character) 0.0))

(event Custom|OpenDoor
  (params (DoorIndex :type Integer))
  (if (== DoorIndex (Variables|Default|GetIndexDoor))
    (Audio|PlaySound2D "/Game/Erwan/Content/Audio/Cue/OpenDoorCue.OpenDoorCue" 1.0 1.0 0.0 0 0)
    (bind _value (Timeline|DitherOnTime Play)
      (:Update
        (Rendering|Material|SetScalarParameterValue (Variables|Default|GetDitherMaterial) "Percent" _value :!class /Script/Engine.MaterialInstanceDynamic))
      (:Finished
        (Actor|DestroyActor)))))

(event EventBeginPlay
  (CallFunction|SetDithering)
  (bind _asbp_game_instance (Utilities|Casting|CastToBP_GameInstance (Game|GetGameInstance)))
  (EventDispatchers|BindEventtoOpenDoor _asbp_game_instance (delegate Custom|OpenDoor)))

(fn ConstructionScript)

(fn SetDithering
  (bind _returnvalue (Rendering|Material|CreateDynamicMaterialInstance "/Game/Erwan/Content/Graphics/M_Dithering.M_Dithering" "None" "None" :!class /Script/Engine.KismetMaterialLibrary))
  (bind _output_get (Variables|Default|SetDitherMaterial _returnvalue))
  (Rendering|Material|SetMaterial (Variables|Default|GetDoor) 0 _output_get))