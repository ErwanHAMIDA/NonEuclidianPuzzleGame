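; AC_Handler is an actor component that relays laser hit events to the other BPI_Lasers components on its owner.
; At BeginPlay it caches those components, sets the owner's static meshes to block or overlap the laser trace channel, and, with InvertSystem, calls LaserStopHitting on SC_Emetter components.
; Start and stop hits always update a queue of incoming lasers, but are forwarded only while the handler is unlocked.
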(event EventBeginPlay
  (Utilities|FlowControl|Sequence
    (:then_0
      (bind _output_get (Variables|Default|SetLinkedComponentArray (Class|Actor|GetComponentsbyInterface (Components|GetOwner) "/Game/Erwan/Content/Gameplay/Lasers/BPI_Lasers.BPI_Lasers_C")))
      (Utilities|Array|RemoveItem _output_get self)
      (CallFunction|SetBlockingObject))
    (:then_1
      (if (Variables|Default|GetInvertSystem)
        (for _array_element (Actor|GetComponentsByClass (Components|GetOwner) "/Game/Erwan/Content/Gameplay/Lasers/SC_Emetter.SC_Emetter_C")
          (Default|LaserStopHitting _array_element))))))

(event EventLaserStopHitting
  (params (Input :type BP%20Laser%20Object%20Reference))
  (CallFunction|LaserRemoved Input)
  (Utilities|IsNotLocked
    (:Not%20Locked
      (bind _array_element (Utilities|ForEachComponent)
        (:LoopBody
          (Class|BPILasers|LaserStopHitting(Message) _array_element Input))))))

(event EventLaserStartHitting
  (params (Input :type BP%20Laser%20Object%20Reference) (HitInfo :type Hit%20Result%20Structure))
  (CallFunction|LaserAdded Input)
  (Utilities|IsNotLocked
    (:Not%20Locked
      (bind _array_element (Utilities|ForEachComponent)
        (:LoopBody
          (Class|BPILasers|LaserStartHitting(Message) _array_element Input HitInfo))))))

(fn LaserAdded
  (params (NewItem :type BP%20Laser%20Object%20Reference%20%28by%20ref%29))
  (Utilities|Array|AddUnique (Variables|Default|GetLaserArrayInQueue) NewItem))

(fn LaserRemoved
  (params (NewItem :type BP%20Laser%20Object%20Reference%20%28by%20ref%29))
  (Utilities|Array|RemoveItem (Variables|Default|GetLaserArrayInQueue) NewItem))

(fn SetBlockingObject
  (for _array_element (Actor|GetComponentsByClass (Components|GetOwner) "/Script/Engine.StaticMeshComponent")
    (Collision|SetCollisionResponsetoChannel _array_element "ECC_GameTraceChannel1" (select (Variables|Conditions|GetIsBlocking) "ECR_Block" "ECR_Overlap"))))