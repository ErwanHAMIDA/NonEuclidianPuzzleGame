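; BP_Laser is a colored laser beam that traces for hits, notifies AC_Handler components and opens doors through laser receptors.
; A looping timer runs a multi-line trace, scaling the mesh to the blocking hit or full range.
; Set differences between trace passes drive handler start/stop messages, filtered by a check against previous lasers.
; Receptor hits call the GameInstance with a door index, and LaserStopHitting notifies handlers before destroying the beam.
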(event Custom|LaserExpand
  (bind (_returnvalue _returnvalue2) (Utilities|StartandEndValues))
  (bind (_outhits _returnvalue_2) (Collision|MultiLineTraceByChannel _returnvalue _returnvalue2 "TraceTypeQuery3" false (Variables|Default|GetActorArrayToIgnore) "None" true "(R=1.000000,G=0.000000,B=0.000000,A=1.000000)" "(R=0.000000,G=1.000000,B=0.000000,A=1.000000)" 1.0))
  (if _returnvalue_2
    (for _array_element _outhits
      (Utilities|FlowControl|Sequence
        (:then_0
          (Utilities|IfBlockUpdateLength (.bBlockingHit (Collision|BreakHitResult _array_element)) (.Distance (Collision|BreakHitResult _array_element))))
        (:then_1
          (CallFunction|HandleHitActors _array_element))
        (:then_2
          (if (Utilities|DoesObjectImplementInterface (.HitActor (Collision|BreakHitResult _array_element)) "/Game/Erwan/Content/Interfaces/BPI_LaserReceptor.BPI_LaserReceptor_C")
            (if (not (Variables|Default|GetIsLaserReceptorTriggered))
              (bind _asbp_laser_receptor (Utilities|Casting|CastToBP_LaserReceptor (.HitActor (Collision|BreakHitResult _array_element))))
              (bind _asbp_game_instance (Utilities|Casting|CastToBP_GameInstance (Game|GetGameInstance)))
              (Variables|Default|SetIsLaserReceptorTriggered true)
              (Default|CallOpenDoor _asbp_game_instance (Variables|/Game/Erwan/Content/Gameplay/Lasers/BP_LaserReceptor.BP_LaserReceptor_C|GetDoorIndex _asbp_laser_receptor)))
            (else
              (Variables|Default|SetIsLaserReceptorTriggered false))))))
    (bind _result (Utilities|Set|Difference (Variables|Default|GetPreviouslyHitHandlerSet) (Variables|Default|GetCurrentHitHandlers)))
    (bind _result_2 (Utilities|Set|ToArray _result))
    (for _array_element_2 _result_2
      (Utilities|Map|Remove (Variables|Default|GetHittingHandlerMap) _array_element_2)
      (Class|BPILasers|LaserStopHitting(Message) _array_element_2 self))
    (Variables|Default|SetPreviouslyHitHandlerSet (Variables|Default|GetCurrentHitHandlers))
    (Utilities|Set|Clear (Variables|Default|GetCurrentHitHandlers))
    (else
      (CallFunction|UpdateLength (Variables|Default|GetRange)))))

(event EventBeginPlay
  (bind _returnvalue (Rendering|Material|CreateDynamicMaterialInstance "/Game/Erwan/Content/Graphics/MI_Laser.MI_Laser" "None" "None" :!class /Script/Engine.KismetMaterialLibrary))
  (bind _output_get (Variables|Default|SetMaterialInstance _returnvalue))
  (Rendering|Material|SetMaterial (Variables|Default|GetLaserMesh) 0 _output_get)
  (CallFunction|ChangeLaserColor (Variables|Exposed|GetColorOverride))
  (Utilities|Time|SetTimerbyEvent (delegate Custom|LaserExpand) 0.1 true))

(event EventLaserStopHitting
  (params (Input :type BP%20Laser%20Object%20Reference))
  (Utilities|FlowControl|Sequence
    (:then_0
      (bind _result (Utilities|Set|ToArray (Variables|Default|GetPreviouslyHitHandlerSet)))
      (for _array_element _result
        (Class|BPILasers|LaserStopHitting(Message) _array_element self)))
    (:then_1
      (Actor|DestroyActor))))

(fn ConstructionScript)

(fn ChangeLaserColor
  (params (Value :type Linear%20Color%20Structure))
  (Rendering|Material|SetVectorParameterValue (Variables|Default|GetMaterialInstance) "Color" Value :!class /Script/Engine.MaterialInstanceDynamic))

(fn UpdateLength
  (params (InputPin :type Float%20%28single-precision%29))
  (if (not (Math|Float|NearlyEqual(Float) InputPin (Variables|Default|GetPreviousLength) 2.0))
    (bind _output_get (Variables|Default|SetPreviousLength InputPin))
    (Transformation|SetWorldScale3D (Variables|Default|GetLaserMesh) (Math|Vector|MakeVector 0.1 0.1 (/ _output_get 195.0)))))

(fn HandleHitActors
  (params (InputPin :type Hit%20Result%20Structure))
  (bind _hitactor (Collision|BreakHitResult InputPin))
  (bind _returnvalue (Actor|GetComponentbyClass _hitactor "/Game/Erwan/Content/Gameplay/Lasers/AC_Handler.AC_Handler_C"))
  (Utilities|IsValid _returnvalue
    (:Is%20Valid
      (bind _output_get (LocalVariables|SetL-Handler _returnvalue))
      (if (CallFunction|IsNotonPath _output_get)
        (Utilities|Map|Add (Variables|Default|GetHittingHandlerMap) (LocalVariables|GetL-Handler) InputPin)
        (if (Utilities|Set|Contains (Variables|Default|GetPreviouslyHitHandlerSet) (LocalVariables|GetL-Handler))
          _
          (else
            (Class|BPILasers|LaserStartHitting(Message) (LocalVariables|GetL-Handler) self InputPin)))
        (Utilities|Set|Add (Variables|Default|GetCurrentHitHandlers) (LocalVariables|GetL-Handler))))))

(fn IsNotonPath
  (params (InputHandler :type AC%20Handler%20Object%20Reference))
  (if (Utilities|Array|IsNotEmpty (Variables|Default|GetPreviousLaserArray))
    (for _array_element (Variables|Default|GetPreviousLaserArray)
      (bind _output_get (LocalVariables|SetL-CurrentLaser _array_element))
      (if true
        (return false)
        (elif (not (CallFunction|IsNotonPath (LocalVariables|GetL-CurrentLaser) InputHandler))
          (return false)))))
  (return true))