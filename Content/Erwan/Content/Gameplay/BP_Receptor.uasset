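; BP_Receptor is a one-shot receptacle that opens an indexed door when an actor implementing BPI_OpenDoor overlaps its box.
; On first activation it plays a validation sound and passes its door index to BP_GameInstance's CallOpenDoor.
; A timeline then offsets the Parent component along Z, and on completion turns the four cubes gathered in the construction script red.
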(event OnComponentBeginOverlap(Box)
  (params (OverlappedComponent :type Primitive%20Component%20Object%20Reference) (OtherActor :type Actor%20Object%20Reference) (OtherComp :type Primitive%20Component%20Object%20Reference) (OtherBodyIndex :type Integer) (bFromSweep :type Boolean) (SweepResult :type Hit%20Result%20Structure%20%28by%20ref%29))
  (if (and (Utilities|DoesObjectImplementInterface OtherActor "/Game/Erwan/Content/Interfaces/BPI_OpenDoor.BPI_OpenDoor_C") (not (Variables|Default|GetIsAlreadyActivated)))
    (Variables|Default|SetIsAlreadyActivated true)
    (Audio|PlaySound2D "/Game/Erwan/Content/Audio/Cue/ReceptacleValidationCue.ReceptacleValidationCue" 1.0 1.0 0.0 0 0)
    (bind _asbp_game_instance (Utilities|Casting|CastToBP_GameInstance (Game|GetGameInstance)))
    (Default|CallOpenDoor _asbp_game_instance (Variables|Default|GetIndexDoor))
    (bind _offset (Timeline|TransitionLocation Play)
      (:Update
        (Transformation|SetRelativeLocation (.Parent (Utilities|ChangeZVector _offset)) (.ReturnValue (Utilities|ChangeZVector _offset)) false false))
      (:Finished
        (CallFunction|SetMaterialonCubes)))))

(event EventBeginPlay)

(event EventTick
  (params (DeltaSeconds :type Float%20%28single-precision%29)))

(fn ConstructionScript
  (Variables|Default|SetCubes (Utilities|Array|MakeArray (Variables|Default|GetCube) (Variables|Default|GetCube1) (Variables|Default|GetCube2) (Variables|Default|GetCube3))))

(fn SetMaterialonCubes
  (for _array_element (Variables|Default|GetCubes)
    (Rendering|Material|SetMaterial _array_element 0 "/Game/Erwan/Content/Graphics/M_Red.M_Red")))

(fn Open
  (params (DoorIndex :type Integer)))